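; Game mode for MaskItOut that times a run and maintains a ranked high-score table in the game instance.
; Tick computes and prints the time elapsed since StartTimer.
; Win inserts that time in ascending order, trims the list at MaxIndex and opens a name-entry widget for qualifying times.
; SaveMapScore stores the name and formatted time at the same index in parallel arrays.
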(event `self.ReceiveBeginPlay`
  (`KismetSystemLibrary.Delay` 0.2)
  (set `self.As GI Mask In Out` (`/Game/Utils/BPL_Utils.GetMaskInOutGI`)))

(event `StartTimer`
  ; start timer
  (set `self.DeltaTime` (`KismetSystemLibrary.GetGameTimeInSeconds`)))

(event `self.ReceiveTick`
  (params (DeltaSeconds :type "Float (single-precision)"))
  (bind _returnvalue (- (`KismetSystemLibrary.GetGameTimeInSeconds`) (`self.DeltaTime`)))
  (bind (_days _hours _minutes _seconds _milliseconds) (`KismetMathLibrary.BreakTimespan` (`KismetMathLibrary.FromSeconds` _returnvalue)))
  (bind _returnvalue_2 (`KismetStringLibrary.Concat_StrStr` (`KismetTextLibrary.Conv_TextToString` (`KismetTextLibrary.Conv_DoubleToText` (`KismetMathLibrary.Conv_IntToDouble` _minutes) "HalfToEven" false true 2)) ":" (`KismetTextLibrary.Conv_TextToString` (`KismetTextLibrary.Conv_DoubleToText` (`KismetMathLibrary.Conv_IntToDouble` _seconds) "HalfToEven" false true 2)) ":" (`KismetTextLibrary.Conv_TextToString` (`KismetTextLibrary.Conv_DoubleToText` (`KismetMathLibrary.Conv_IntToDouble` _milliseconds) "HalfToEven" false true 3 3))))
  ; calculate time
  (set `self.TimeFloat` _returnvalue)
  (set `self.Time` _returnvalue_2)
  (`KismetSystemLibrary.PrintString` _returnvalue_2 true true (struct :`G` 0.66 :`B` 1.0 :`A` 1.0) 2.0 "timer"))

(event `BreakLoop`
  (bind _scorelist (`/Game/Managers/GI_MaskInOut.ScoreList` (`self.As GI Mask In Out`)))
  (goto _label :!via `Break`))

(event `Win`
  (bind _scorelist (`/Game/Managers/GI_MaskInOut.ScoreList` (`self.As GI Mask In Out`)))
  (if (> (`KismetArrayLibrary.Array_Length` (`/Game/Managers/GI_MaskInOut.ScoreList` (`self.As GI Mask In Out`))) 0)
    (bind _output_get (set `self.CopyScore` (`/Game/Managers/GI_MaskInOut.ScoreList` (`self.As GI Mask In Out`))))
    (for (_array_element _array_index) _output_get :!label _label
      (if (< (`self.TimeFloat`) _array_element)
        (`KismetArrayLibrary.Array_Insert` (`/Game/Managers/GI_MaskInOut.ScoreList` (`self.As GI Mask In Out`)) (`self.TimeFloat`) _array_index)
        (set `self.IndexName` _array_index)
        (`self.CanvasInsertScore`)
        (set `self.InsertInMiddle` true)
        (`self.BreakLoop`)))
    (if (`self.InsertInMiddle`)
      (set `self.InsertInMiddle` false)
      (else
        (bind _output_get_2 (set `self.IndexName` (+ (`KismetArrayLibrary.Array_LastIndex` _scorelist) 1)))
        (`KismetArrayLibrary.Array_Insert` _scorelist (`self.TimeFloat`) _output_get_2)))
    (if (> (`KismetArrayLibrary.Array_Length` (`/Game/Managers/GI_MaskInOut.ScoreList` (`self.As GI Mask In Out`))) (`self.MaxIndex`))
      (`KismetArrayLibrary.Array_Remove` (`/Game/Managers/GI_MaskInOut.ScoreList` (`self.As GI Mask In Out`)) (`self.MaxIndex`))
      (else
        (`self.CanvasInsertScore`)))
    (else
      (bind _returnvalue (`KismetArrayLibrary.Array_Add` (`/Game/Managers/GI_MaskInOut.ScoreList` (`self.As GI Mask In Out`)) (`self.TimeFloat`)))
      (set `self.IndexName` _returnvalue)
      (`self.CanvasInsertScore`))))

(event `SaveMapScore`
  (params (NameToSave :type "String (by ref)"))
  (`KismetArrayLibrary.Array_Insert` (`/Game/Managers/GI_MaskInOut.ScoreName` (`self.As GI Mask In Out`)) NameToSave (`self.IndexName`))
  (`KismetArrayLibrary.Array_Insert` (`/Game/Managers/GI_MaskInOut.ScoreUnitString` (`self.As GI Mask In Out`)) (`self.Time`) (`self.IndexName`))
  (if (> (`KismetArrayLibrary.Array_Length` (`/Game/Managers/GI_MaskInOut.ScoreUnitString` (`self.As GI Mask In Out`))) (`self.MaxIndex`))
    (`KismetArrayLibrary.Array_Remove` (`/Game/Managers/GI_MaskInOut.ScoreUnitString` (`self.As GI Mask In Out`)) (`self.MaxIndex`))
    (`KismetArrayLibrary.Array_Remove` (`/Game/Managers/GI_MaskInOut.ScoreName` (`self.As GI Mask In Out`)) (`self.MaxIndex`))))

(event `CanvasInsertScore`
  (bind _returnvalue (`GameplayStatics.GetPlayerController` 0))
  (bind _returnvalue_2 (`|CreateWidget` "/Game/Widgets/BPW_InsertName.BPW_InsertName_C"))
  (`/Game/Widgets/BPW_InsertName.SetTime` _returnvalue_2 (`self.Time`))
  (`UserWidget.AddToViewport` _returnvalue_2 0)
  (set `PlayerController.bShowMouseCursor` true _returnvalue)
  (`WidgetBlueprintLibrary.SetInputMode_GameAndUIEx` _returnvalue _returnvalue_2 "DoNotLock" false true))

(fn `UserConstructionScript`)