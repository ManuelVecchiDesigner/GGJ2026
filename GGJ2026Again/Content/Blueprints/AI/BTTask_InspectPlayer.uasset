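; Behavior Tree task that sends the AI pawn to inspect the player, getting closer as suspicion escalates.
; It stops current movement, queries the pawn's inspection status and runs AI MoveTo toward the blackboard Player with a status-dependent acceptance radius.
; On arrival it prints a debug message, sets IsCaught for the Get Caught status and finishes successfully.
; A failed move has no handler, so the task never finishes in that case.
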(event `self.ReceiveExecuteAI`
  (params (OwnerController :type "AIController Object Reference") (ControlledPawn :type "Pawn Object Reference"))
  (`MovementComponent.StopMovementImmediately` (`Character.CharacterMovement` (cast `Character` ControlledPawn :!pure true)))
  (bind _inspection_status (message `/Game/Blueprints/AI/BPI_Guard.GetInspectionStatus` ControlledPawn))
  (`|AIMoveTo` ControlledPawn (0.0 0.0 0.0) (`BTFunctionLibrary.GetBlackboardValueAsActor` (`self.Player`)) (select `/Game/Blueprints/AI/E_InspectionStatus` _inspection_status :`NewEnumerator0` 500.0 :`NewEnumerator1` 350.0 :`NewEnumerator2` 100.0 :`NewEnumerator3` 20.0 :!type "Float (single-precision)")
    (:`OnSuccess`
      (`KismetSystemLibrary.PrintString` (select `/Game/Blueprints/AI/E_InspectionStatus` _inspection_status :`NewEnumerator0` "First time low suspicious" :`NewEnumerator1` "second time normal suspicious" :`NewEnumerator2` "third time susper suspicious" :`NewEnumerator3` "call get caught"))
      (switch `/Game/Blueprints/AI/E_InspectionStatus` _inspection_status
        (:`NewEnumerator0`
          _)
        (:`NewEnumerator1`
          _)
        (:`NewEnumerator2`
          _)
        (:`NewEnumerator3`
          (`BTFunctionLibrary.SetBlackboardValueAsBool` (`self.isCaught?`) true)))
      (`self.FinishExecute` true))))