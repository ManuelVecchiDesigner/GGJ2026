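; BP_HideZone is a trigger volume that lets the player hide when wearing the mask the zone requests.
; On box overlap, it reads the current mask through BPI_Player, compares it to MaskRequested and sends the result back as the can-hide state.
; The mask is checked only on entry, with a debug print of the result.
; Leaving the box sends a can-hide false message to the exiting actor.
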(event `self.Box.OnComponentBeginOverlap`
  (params (OverlappedComponent :type "PrimitiveComponent Object Reference") (OtherActor :type "Actor Object Reference") (OtherComp :type "PrimitiveComponent Object Reference") (OtherBodyIndex :type Integer) (bFromSweep :type Boolean) (SweepResult :type "HitResult Structure (by ref)"))
  (bind _maskrequested (`self.MaskRequested`))
  (if (`KismetSystemLibrary.DoesImplementInterface` OtherActor "/Game/Blueprints/Player/BPI_Player.BPI_Player_C")
    (bind _currentmask (message `/Game/Blueprints/Player/BPI_Player.GetCurrentMask` OtherActor))
    (bind _returnvalue (`|EnumEquality` _currentmask _maskrequested))
    (message `/Game/Blueprints/Player/BPI_Player.SetCanHide` OtherActor _returnvalue)
    (`KismetSystemLibrary.PrintString` (`KismetStringLibrary.Concat_StrStr` "Player has " (`|GetEnumeratorNameAsString` _currentmask) " mask requested is " (`|GetEnumeratorNameAsString` _maskrequested) " player can hide " (`KismetStringLibrary.Conv_BoolToString` _returnvalue)))))

(event `self.Box.OnComponentEndOverlap`
  (params (OverlappedComponent :type "PrimitiveComponent Object Reference") (OtherActor :type "Actor Object Reference") (OtherComp :type "PrimitiveComponent Object Reference") (OtherBodyIndex :type Integer))
  (message `/Game/Blueprints/Player/BPI_Player.SetCanHide` OtherActor false))

(fn `UserConstructionScript`)