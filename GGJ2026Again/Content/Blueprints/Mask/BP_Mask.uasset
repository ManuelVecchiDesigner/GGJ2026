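; BP_Mask is a mask pickup actor that bobs and spins in the world and shows a widget while overlapped.
; Two timelines, rate-scaled by MovementTime, drive the mesh's height and yaw from its starting transform.
; Sphere overlaps pass the mask to the other actor and clear it on exit, with Pawn overlap held off for one second after BeginPlay.
; DisappearFromWord hides the mesh and disables collision instead of destroying the actor.
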(event `self.ReceiveBeginPlay`
  (bind _mesh_mask (`self.Mesh_Mask`))
  (`PrimitiveComponent.SetCollisionResponseToChannel` (`self.SphereCollision`) "ECC_Pawn" "ECR_Ignore")
  (set `self.StartZ` (.z (`SceneComponent.RelativeLocation` _mesh_mask)))
  (set `self.StartYaw` (.yaw (`SceneComponent.RelativeRotation` _mesh_mask)))
  (`TimelineComponent.SetPlayRate` (`self.MaskMovement`) (/ 1.0 (`self.MovementTime`)))
  (`TimelineComponent.SetPlayRate` (`self.rotation`) (/ 1.0 (`self.MovementTime`)))
  (`TimelineComponent.PlayFromStart` (`self.MaskMovement`))
  (`TimelineComponent.PlayFromStart` (`self.rotation`))
  (`KismetSystemLibrary.Delay` 1.0)
  (`PrimitiveComponent.SetCollisionResponseToChannel` (`self.SphereCollision`) "ECC_Pawn" "ECR_Overlap"))

(event `self.SphereCollision.OnComponentBeginOverlap`
  (params (OverlappedComponent :type "PrimitiveComponent Object Reference") (OtherActor :type "Actor Object Reference") (OtherComp :type "PrimitiveComponent Object Reference") (OtherBodyIndex :type Integer) (bFromSweep :type Boolean) (SweepResult :type "HitResult Structure (by ref)"))
  (message `/Game/Blueprints/Player/BPI_Player.PassMask` OtherActor self)
  (`SceneComponent.SetVisibility` (`self.Widget`) true false))

(event `self.SphereCollision.OnComponentEndOverlap`
  (params (OverlappedComponent :type "PrimitiveComponent Object Reference") (OtherActor :type "Actor Object Reference") (OtherComp :type "PrimitiveComponent Object Reference") (OtherBodyIndex :type Integer))
  (message `/Game/Blueprints/Player/BPI_Player.PassMask` OtherActor null)
  (`SceneComponent.SetVisibility` (`self.Widget`) false false))

(event `DisappearFromWord`
  (`PrimitiveComponent.SetCollisionResponseToAllChannels` (`self.SphereCollision`) "ECR_Ignore")
  (`SceneComponent.SetVisibility` (`self.Mesh_Mask`) false false))

(fn `UserConstructionScript`)